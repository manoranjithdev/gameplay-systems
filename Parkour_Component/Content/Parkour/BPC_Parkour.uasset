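; Character parkour component that climbs, mantles or vaults obstacles when Do_Parkour fires, unless a montage is playing or the character is falling.
; A forward sphere trace finds the obstacle, then downward traces measure its top and depth to pick the action and montage.
; Motion Warping, added at BeginPlay, aligns the montage using offset targets.
; The capsule loses collision and movement switches to Flying until the montage blends out or is interrupted.
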(event `self.ReceiveBeginPlay`
  (bind _ascharacter (cast `Character` (`self.GetOwner`)))
  (set `self.As Character` _ascharacter)
  (bind _returnvalue (`|AddComponentByClass` (`self.As Character`) "/Script/MotionWarping.MotionWarpingComponent"))
  (set `self.Motion warping` _returnvalue))

(event `Do_Parkour`
  (if (not (or (`AnimInstance.IsAnyMontagePlaying` (`SkeletalMeshComponent.GetAnimInstance` (`Character.Mesh` (`self.As Character`)))) (`NavMovementComponent.IsFalling` (`Character.CharacterMovement` (`self.As Character`)))))
    ; Check for Parkour Obstacle and proceed when Found
    (`self.Obstacle detection`)
    (if (`self.Obstacle Detected`)
      ; Fuction to measure the parkour obstacle
      (`self.Obstacle Query`)
      ; Desired parkour action based on measurement from obstacle query
      (`self.Obstacle Action`)
      ; Proceed if parkour action is decided
      (if (not (`|EnumEquality` (`self.Parkour action`) "NewEnumerator0"))
        (`self.Character Settings` "NoCollision" "MOVE_Flying")
        (`self.Set Motion Warping Targets`)
        (`|PlayMontage` (`Character.Mesh` (`self.As Character`)) (`self.Montage to Play`)
          (:`OnBlendOut`
            _)
          (:`OnInterrupted`
            _))
        (`self.Character Settings` "QueryAndPhysics" "MOVE_Walking")))))

(fn `Character Settings`
  (params (NewCollision :type "ECollisionEnabled Enum" :default "NoCollision") (NewMovementMode :type "EMovementMode Enum" :default "MOVE_None"))
  (`PrimitiveComponent.SetCollisionEnabled` (`Character.CapsuleComponent` (`self.As Character`)) NewCollision)
  (`CharacterMovementComponent.SetMovementMode` (`Character.CharacterMovement` (`self.As Character`)) NewMovementMode 0))

(fn `Obstacle Action`
  (if (`self.Is Parkour obstacle valid`)
    (bind _height (`self.Obstacle height`))
    (if (> _height (`self.Climb Height`))
      (set `self.Parkour action` "NewEnumerator1")
      (set `self.Montage to Play` (`self.Climb Montage`))
      (elif (`self.Is Obstacle Deep`)
        (set `self.Parkour action` "NewEnumerator2")
        (set `self.Montage to Play` (`self.Mantle Montage`))
        (else
          (set `self.Parkour action` "NewEnumerator3")
          (set `self.Montage to Play` (`self.Vault Montage`)))))
    (else
      (set `self.Parkour action` "NewEnumerator0"))))

(fn `Obstacle detection`
  ; Ths is the first trace that checks for obstacle using custom collision
  (bind _outhit (`KismetSystemLibrary.SphereTraceSingleForObjects` (`Actor.K2_GetActorLocation` (`self.As Character`)) (+ (`Actor.K2_GetActorLocation` (`self.As Character`)) (* (`KismetMathLibrary.GetForwardVector` (`Actor.K2_GetActorRotation` (`self.As Character`))) 120.0)) 20.0 (`|MakeArray` (`self.Obstacle Detection Channel`))))
  (bind (_bblockinghit _binitialoverlap _time _distance _location _impactpoint _normal _impactnormal) (`GameplayStatics.BreakHitResult` _outhit))
  (set `self.Obstacle Detected` _bblockinghit)
  (set `self.Obstacle detected location` _impactpoint)
  (bind (_returnvalue_roll _returnvalue_pitch _returnvalue_yaw) (`KismetMathLibrary.BreakRotator` (`KismetMathLibrary.NormalizedDeltaRotator` (`KismetMathLibrary.MakeRotFromX` _impactnormal) (struct :`Yaw` 180.0))))
  (set `self.Obstacle Rotation` (`KismetMathLibrary.MakeRotator` 0.0 0.0 _returnvalue_yaw)))

(fn `Obstacle height`
  (returns (Height :type "Float (double-precision)"))
  (bind (_returnvalue_x _returnvalue_y _returnvalue_z) (`KismetMathLibrary.BreakVector` (- (`self.Obstacle Start Location`) (`SceneComponent.GetSocketLocation` (`Character.Mesh` (`self.As Character`)) "root"))))
  (return _returnvalue_z))

(fn `Obstacle Query`
  (bind _returnvalue (+ (* (`KismetMathLibrary.GetForwardVector` (`self.Obstacle Rotation`)) 65.0) (`self.Obstacle Start Location`)))
  ; Second trace to get obstacle top location, and obstacle validation for parkour
  (bind _outhit (`KismetSystemLibrary.SphereTraceSingle` (+ (`self.Obstacle detected location`) (0.0 0.0 200.0)) (- (`self.Obstacle detected location`) (0.0 0.0 10.0)) 25.0 "TraceTypeQuery1"))
  (bind (_bblockinghit _binitialoverlap _time _distance _location _impactpoint) (`GameplayStatics.BreakHitResult` _outhit))
  (set `self.Is Parkour obstacle valid` (and _bblockinghit (not _binitialoverlap)))
  (set `self.Obstacle Start Location` _impactpoint)
  ; Third trace to calculate the obstacle depth
  (bind _outhit_2 (`KismetSystemLibrary.SphereTraceSingle` _returnvalue (- _returnvalue (0.0 0.0 250.0)) 15.0 "TraceTypeQuery1"))
  (bind (_bblockinghit_2 _binitialoverlap_2 _time_2 _distance_2 _location_2 _impactpoint_2 _normal _impactnormal _physmat _hitactor _hitcomponent _hitbonename _bonename _hititem _elementindex _faceindex _tracestart _traceend) (`GameplayStatics.BreakHitResult` _outhit_2))
  (set `self.Is Obstacle Deep` _binitialoverlap_2)
  (set `self.Obstacle End Location` (`KismetMathLibrary.SelectVector` _impactpoint_2 _traceend _bblockinghit_2)))

(fn `Set Motion Warping Targets`
  (switch `/Game/Parkour/E_Parkour` (`self.Parkour action`)
    (:`NewEnumerator1`
      (bind _location_out (`self.Warp Offset` (`self.Obstacle Start Location`) (`self.Climb Forward Offset`) (`self.Climb Up Offset`)))
      (`MotionWarpingComponent.AddOrUpdateWarpTargetFromLocationAndRotation` (`self.Motion warping`) "Start" _location_out (`self.Obstacle Rotation`))
      (bind _location_out_2 (`self.Warp Offset` (`self.Obstacle Start Location`) (`self.Climb end Forward Offset`) (`self.Climb End Up Offset`)))
      (`MotionWarpingComponent.AddOrUpdateWarpTargetFromLocationAndRotation` (`self.Motion warping`) "None" _location_out_2 (`self.Obstacle Rotation`)))
    (:`NewEnumerator2`
      (bind _location_out_3 (`self.Warp Offset` (`self.Obstacle Start Location`) (`self.Mantle Forward Offset`) (`self.Mantle Up Offset`)))
      (`MotionWarpingComponent.AddOrUpdateWarpTargetFromLocationAndRotation` (`self.Motion warping`) "Start" _location_out_3 (`self.Obstacle Rotation`))
      (bind _location_out_4 (`self.Warp Offset` (`self.Obstacle End Location`) (`self.End Forward Offset`) (`self.End Up Offset`)))
      (`MotionWarpingComponent.AddOrUpdateWarpTargetFromLocationAndRotation` (`self.Motion warping`) "None" _location_out_4 (`self.Obstacle Rotation`)))
    (:`NewEnumerator3`
      (bind _location_out_5 (`self.Warp Offset` (`self.Obstacle Start Location`) (`self.Vault Forward Offset`) (`self.Vault Up Offset`)))
      (`MotionWarpingComponent.AddOrUpdateWarpTargetFromLocationAndRotation` (`self.Motion warping`) "Start" _location_out_5 (`self.Obstacle Rotation`))
      (bind _location_out_6 (`self.Warp Offset` (`self.Obstacle End Location`) (`self.End Vault Forward Offset`) (`self.End Vault Up Offset`)))
      (`MotionWarpingComponent.AddOrUpdateWarpTargetFromLocationAndRotation` (`self.Motion warping`) "None" _location_out_6 (`self.Obstacle Rotation`)))))

(fn `Warp Offset`
  (params (`Location in` :type "Vector Structure") (`Forward Offset` :type "Float (double-precision)") (`Up Offset` :type "Float (double-precision)"))
  (returns (`Location out` :type "Vector Structure"))
  (return (+ (+ `Location in` (`KismetMathLibrary.MakeVector` 0.0 0.0 `Up Offset`)) (* (`KismetMathLibrary.GetForwardVector` (`self.Obstacle Rotation`)) `Forward Offset`))))