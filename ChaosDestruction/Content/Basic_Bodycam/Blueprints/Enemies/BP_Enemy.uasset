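; Enemy Blueprint that tracks health, spills blood when damaged and ragdolls on death.
; AnyDamage subtracts from Health, which starts at MaxHealth, and calls SpawnBlood on non-lethal hits.
; At zero health, DoOnce-gated logic removes the capsule, enables mesh physics, changes its stencil value, plays a random death scream and pushes the body along the player's forward vector.
; SpawnBlood traces from four arrow components and attaches randomly sized decals.
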(event `self.ReceiveAnyDamage`
  (params (Damage :type "Float (single-precision)") (DamageType :type "DamageType Object Reference") (InstigatedBy :type "Controller Object Reference") (DamageCauser :type "Actor Object Reference"))
  ;[0.01998 0.15 0 0.5] TAKING DAMAGE
  (bind _output_get (set `self.health` (- (`self.health`) Damage)))
  (if (<= _output_get 0.0)
    (`|ExecutionSequence`
      (:`then_0`
        (`/Engine/EditorBlueprintResources/StandardMacros.DoOnce` false
          (:`Completed`
            (`ActorComponent.K2_DestroyComponent` (`self.CapsuleComponent`))
            (`PrimitiveComponent.SetSimulatePhysics` (`self.Mesh`) true)
            (`PrimitiveComponent.SetCustomDepthStencilValue` (`self.Mesh`) 10)
            (`|ExecutionSequence`
              (:`then_0`
                (switch `int` (`KismetMathLibrary.RandomIntegerInRange` 0 4)
                  (:`0`
                    (`GameplayStatics.PlaySoundAtLocation` "/Game/Basic_Bodycam/Sounds/SW_Death2.SW_Death2" (`self.K2_GetActorLocation`) (struct) 0.45 1.0 0.0 "/Game/Basic_Bodycam/Sounds/SA_Gunshot.SA_Gunshot" null null null))
                  (:`1`
                    (`GameplayStatics.PlaySoundAtLocation` "/Game/Basic_Bodycam/Sounds/SW_Death4.SW_Death4" (`self.K2_GetActorLocation`) (struct) 0.45 1.0 0.0 "/Game/Basic_Bodycam/Sounds/SA_Gunshot.SA_Gunshot" null null null))
                  (:`2`
                    (`GameplayStatics.PlaySoundAtLocation` "/Game/Basic_Bodycam/Sounds/SW_Death1.SW_Death1" (`self.K2_GetActorLocation`) (struct) 0.45 1.0 0.0 "/Game/Basic_Bodycam/Sounds/SA_Gunshot.SA_Gunshot" null null null))
                  (:`3`
                    (`GameplayStatics.PlaySoundAtLocation` "/Game/Basic_Bodycam/Sounds/SW_Death5.SW_Death5" (`self.K2_GetActorLocation`) (struct) 0.45 1.0 0.0 "/Game/Basic_Bodycam/Sounds/SA_Gunshot.SA_Gunshot" null null null))
                  (:`4`
                    (`GameplayStatics.PlaySoundAtLocation` "/Game/Basic_Bodycam/Sounds/SW_Death3.SW_Death3" (`self.K2_GetActorLocation`) (struct) 0.45 1.0 0.0 "/Game/Basic_Bodycam/Sounds/SA_Gunshot.SA_Gunshot" null null null))))
              (:`then_1`
                (goto _label :!via `Reset`))
              (:`then_2`
                (`self.Spawn Blood`))))))
      (:`then_1`
        (`/Engine/EditorBlueprintResources/StandardMacros.DoOnce` true :!label _label
          (:`Completed`
            (bind _asbp_first_person_character (cast `/Game/Basic_Bodycam/Blueprints/Player/BP_FP_Character` (`GameplayStatics.GetPlayerCharacter` 0)))
            (`PrimitiveComponent.AddImpulse` (`self.Mesh`) (* (`self.GetActorForwardVector` _asbp_first_person_character) 500.0) "None" true)
            (goto _label :!via `Reset`)))))
    (else
      (`self.Spawn Blood`))))

(event `self.ReceiveBeginPlay`
  ;[1 1 1] EVENT BEGIN PLAY
  (set `self.health` (`self.maxHealth`)))

(event `Spawn Blood`
  (bind _arrow1 (`self.Arrow1`))
  (bind _arrow2 (`self.Arrow2`))
  (bind _arrow3 (`self.Arrow3`))
  (bind _arrow4 (`self.Arrow4`))
  (bind _returnvalue (`SceneComponent.K2_GetComponentLocation` _arrow4))
  (bind _returnvalue_2 (`SceneComponent.K2_GetComponentLocation` _arrow2))
  (bind _returnvalue_3 (`SceneComponent.K2_GetComponentLocation` _arrow3))
  (bind _returnvalue_4 (`SceneComponent.K2_GetComponentLocation` _arrow1))
  ;[1 0.03061 0 0.5] SPAWNING BLOOD
  (`|ExecutionSequence`
    (:`then_0`
      (bind _outhit (`KismetSystemLibrary.LineTraceSingle` _returnvalue_4 (+ _returnvalue_4 (* (`SceneComponent.GetForwardVector` _arrow1) 300.0)) "TraceTypeQuery1"))
      (bind (_bblockinghit _binitialoverlap _time _distance _location _impactpoint _normal _impactnormal _physmat _hitactor _hitcomponent) (`GameplayStatics.BreakHitResult` _outhit))
      (`GameplayStatics.SpawnDecalAttached` "/Game/Basic_Bodycam/Materials/Decals/M_Blood_Decal.M_Blood_Decal" (`KismetMathLibrary.Conv_IntToVector` (`KismetMathLibrary.RandomIntegerInRange` 20 30)) _hitcomponent "None" _location (`KismetMathLibrary.Conv_VectorToRotator` _impactnormal) "KeepWorldPosition" 80.0))
    (:`then_1`
      (bind _outhit_2 (`KismetSystemLibrary.LineTraceSingle` _returnvalue_2 (+ _returnvalue_2 (* (`SceneComponent.GetForwardVector` _arrow2) 300.0)) "TraceTypeQuery1"))
      (bind (_bblockinghit_2 _binitialoverlap_2 _time_2 _distance_2 _location_2 _impactpoint_2 _normal_2 _impactnormal_2 _physmat_2 _hitactor_2 _hitcomponent_2) (`GameplayStatics.BreakHitResult` _outhit_2))
      (`GameplayStatics.SpawnDecalAttached` "/Game/Basic_Bodycam/Materials/Decals/M_Blood_Decal.M_Blood_Decal" (`KismetMathLibrary.Conv_IntToVector` (`KismetMathLibrary.RandomIntegerInRange` 20 30)) _hitcomponent_2 "None" _location_2 (`KismetMathLibrary.Conv_VectorToRotator` _impactnormal_2) "KeepWorldPosition" 80.0))
    (:`then_2`
      (bind _outhit_3 (`KismetSystemLibrary.LineTraceSingle` _returnvalue_3 (+ _returnvalue_3 (* (`SceneComponent.GetForwardVector` _arrow3) 300.0)) "TraceTypeQuery1"))
      (bind (_bblockinghit_3 _binitialoverlap_3 _time_3 _distance_3 _location_3 _impactpoint_3 _normal_3 _impactnormal_3 _physmat_3 _hitactor_3 _hitcomponent_3) (`GameplayStatics.BreakHitResult` _outhit_3))
      (`GameplayStatics.SpawnDecalAttached` "/Game/Basic_Bodycam/Materials/Decals/M_Blood_Decal.M_Blood_Decal" (`KismetMathLibrary.Conv_IntToVector` (`KismetMathLibrary.RandomIntegerInRange` 20 30)) _hitcomponent_3 "None" _location_3 (`KismetMathLibrary.Conv_VectorToRotator` _impactnormal_3) "KeepWorldPosition" 80.0))
    (:`then_3`
      (bind _outhit_4 (`KismetSystemLibrary.LineTraceSingle` _returnvalue (+ _returnvalue (* (`SceneComponent.GetForwardVector` _arrow4) 300.0)) "TraceTypeQuery1"))
      (bind (_bblockinghit_4 _binitialoverlap_4 _time_4 _distance_4 _location_4 _impactpoint_4 _normal_4 _impactnormal_4 _physmat_4 _hitactor_4 _hitcomponent_4) (`GameplayStatics.BreakHitResult` _outhit_4))
      (`GameplayStatics.SpawnDecalAttached` "/Game/Basic_Bodycam/Materials/Decals/M_Blood_Decal.M_Blood_Decal" (`KismetMathLibrary.Conv_IntToVector` (`KismetMathLibrary.RandomIntegerInRange` 20 30)) _hitcomponent_4 "None" _location_4 (`KismetMathLibrary.Conv_VectorToRotator` _impactnormal_4) "KeepWorldPosition" 80.0))))

(fn `UserConstructionScript`)